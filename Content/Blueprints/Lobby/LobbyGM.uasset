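; LobbyGM is the lobby game mode that spawns and possesses a character for each player who logs in.
; PostLogin caches the LobbyPC and GameInfoInstance, then loads PlayerSaveGame from the "PlayerSettingsSave" slot on the machine running the game mode.
; The saved MyPlayerCharacter class is spawned at SpawnLocation, adjusted for collisions, and possessed by the new controller.
; Each login overwrites the single stored controller and save references.
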(event EventPostLogin
  (params (NewPlayer :type Player%20Controller%20Object%20Reference))
  ;[1 1 1] To moznaby wydzielic jako funkcja przygotowujaca wszystkie dane
  ;;[1 1 1] Saving reference to player controller
  (bind _aslobby_pc (Utilities|Casting|CastToLobbyPC NewPlayer))
  (Variables|Default|SetLobby%20Player%20Controller%20Ref _aslobby_pc)
  ;;[1 1 1] Saving reference to game instance
  (bind _asgame_info_instance (Utilities|Casting|CastToGameInfoInstance (Game|GetGameInstance)))
  (Variables|Default|SetGameInstanceRef _asgame_info_instance)
  ;;[1 1 1] Loading and saving SaveGameRef
  (bind _returnvalue (SaveGame|LoadGamefromSlot "PlayerSettingsSave"))
  (bind _asplayer_save_game (Utilities|Casting|CastToPlayerSaveGame _returnvalue))
  (bind _output_get (Variables|Default|SetSaveGameRef _asplayer_save_game))
  ;[1 1 1] Spawn proper actor and let the player controller possess him
  (bind _returnvalue_2 (Game|SpawnActorfromClass (.myplayercharacter (Variables|/Game/Blueprints/AllLevels/PlayerSaveGame.PlayerSaveGame_C|GetS_PlayerInfo _output_get)) (Variables|Default|GetSpawnLocation) "AdjustIfPossibleButAlwaysSpawn" 0 0))
  (Pawn|Possess (Variables|Default|GetLobby%20Player%20Controller%20Ref) _returnvalue_2))

(fn ConstructionScript)