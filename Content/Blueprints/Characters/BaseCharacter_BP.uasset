(event Custom|SpawnProjectile
  (params (ProjectileClass :type Actor%20Class%20Reference))
  ;[1 1 1] Spawns a projectile. This is called by the skill classes because those classes are unable to spawn actors
  (Game|SpawnActorfromClass ProjectileClass (Transformation|GetWorldTransform (Variables|Default|GetProjectileSpawnPoint)) "Undefined" self 0))

(event EventBeginPlay
  (Networking|SwitchHasAuthority
    (:Authority
      (CallFunction|InitAttributes))))

(event Collision|EventActorBeginOverlap
  (params (OtherActor :type Actor%20Object%20Reference)))

(event EventTick
  (params (DeltaSeconds :type Float%20%28single-precision%29)))

(fn ConstructionScript)

(fn OnRepHealth)

(fn InitAttributes
  (Variables|Attributes|SetHealth (Variables|Attributes|GetMaxHealth)))

(fn OnTakeDamage
  (params (DamageTaken :type Float%20%28single-precision%29))
  (Networking|SwitchHasAuthority
    (:Authority
      (bind _output_get (Variables|Attributes|SetHealth (- (Variables|Attributes|GetHealth) DamageTaken)))
      (if (<= _output_get 0.0)
        (CallFunction|OnDeath)))))

(fn OnDeath
  (Rendering|Components|TextRender|SetText (Variables|Default|GetStatus) (Utilities|Text|ToText(String) (Utilities|String|MakeLiteralString "You Died!"))))