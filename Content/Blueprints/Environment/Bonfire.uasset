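; Bonfire environment actor that burns characters who get too close and heals characters resting nearby.
; A looping-style timeline scales the fire light's intensity from its initial value captured in the construction script.
; The inner sphere spawns an explosion on any overlap and damages BaseCharacter_BP actors.
; The healing sphere tracks characters in a list, which the server heals every second by applying negative damage through a DoOnce-and-Delay throttle on Tick.
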(event OnComponentBeginOverlap(HealingSphere)
  (params (OverlappedComponent :type Primitive%20Component%20Object%20Reference) (OtherActor :type Actor%20Object%20Reference) (OtherComp :type Primitive%20Component%20Object%20Reference) (OtherBodyIndex :type Integer) (bFromSweep :type Boolean) (SweepResult :type Hit%20Result%20Structure%20%28by%20ref%29))
  ;[1 1 1] Handle events when character enters healing sphere
  (bind _asbase_character_bp (Utilities|Casting|CastToBaseCharacter_BP OtherActor))
  (Utilities|Array|Add (Variables|Default|GetCharactersToHeal) _asbase_character_bp))

(event OnComponentEndOverlap(HealingSphere)
  (params (OverlappedComponent :type Primitive%20Component%20Object%20Reference) (OtherActor :type Actor%20Object%20Reference) (OtherComp :type Primitive%20Component%20Object%20Reference) (OtherBodyIndex :type Integer))
  ;[1 1 1] Handle events when character enters healing sphere
  (bind _asbase_character_bp (Utilities|Casting|CastToBaseCharacter_BP OtherActor))
  (Utilities|Array|RemoveItem (Variables|Default|GetCharactersToHeal) _asbase_character_bp))

(event OnComponentBeginOverlap(Sphere)
  (params (OverlappedComponent :type Primitive%20Component%20Object%20Reference) (OtherActor :type Actor%20Object%20Reference) (OtherComp :type Primitive%20Component%20Object%20Reference) (OtherBodyIndex :type Integer) (bFromSweep :type Boolean) (SweepResult :type Hit%20Result%20Structure%20%28by%20ref%29))
  ;[1 1 1] Handle events when character get too close to fire
  (Effects|SpawnEmitteratLocation "/Game/StarterContent/Particles/P_Explosion.P_Explosion" (Transformation|GetActorLocation))
  (bind _asbase_character_bp (Utilities|Casting|CastToBaseCharacter_BP OtherActor))
  (Game|Damage|ApplyDamage _asbase_character_bp (Variables|Default|GetDamage) 0 0))

(event EventBeginPlay
  ;[1 1 1] BeginPlay - Changes light intensity over time
  (bind _lightintensity (Timeline|FireIntensity Play)
    (:Update
      (Rendering|Components|Light|SetIntensity (Variables|Default|GetFireLight) (* _lightintensity (Variables|Default|GetInitialIntensity))))))

(event EventTick
  (params (DeltaSeconds :type Float%20%28single-precision%29))
  ;[1 1 1] Tick - Heals characters inside healing sphere (apply damage with "-")
  (Networking|SwitchHasAuthority
    (:Authority
      (Utilities|FlowControl|DoOnce false :!label _label
        (:Completed
          (for _array_element (Variables|Default|GetCharactersToHeal)
            (Game|Damage|ApplyDamage _array_element (- 0.0 (Variables|Default|GetHealingRate)) 0 0))
          (Utilities|FlowControl|Delay 1.0)
          (goto _label Reset))))))

(fn ConstructionScript
  (Variables|Default|SetInitialIntensity (Variables|/Script/Engine.LightComponentBase|GetIntensity (Variables|Default|GetFireLight))))