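; Binfire is an environment hazard actor: a burning bin that flickers and hurts characters who touch it.
; On BeginPlay a FireIntensity timeline scales the point light's intensity against the value cached in the construction script.
; Overlapping its sphere spawns an explosion emitter at the actor's location, then applies damage if the other actor is a BaseCharacter_BP.
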(event OnComponentBeginOverlap(Sphere)
  (params (OverlappedComponent :type Primitive%20Component%20Object%20Reference) (OtherActor :type Actor%20Object%20Reference) (OtherComp :type Primitive%20Component%20Object%20Reference) (OtherBodyIndex :type Integer) (bFromSweep :type Boolean) (SweepResult :type Hit%20Result%20Structure%20%28by%20ref%29))
  (Effects|SpawnEmitteratLocation "/Game/StarterContent/Particles/P_Explosion.P_Explosion" (Transformation|GetActorLocation))
  (bind _asbase_character_bp (Utilities|Casting|CastToBaseCharacter_BP OtherActor))
  (Game|Damage|ApplyDamage _asbase_character_bp (Variables|Default|GetDamage) 0 0))

(event EventBeginPlay
  (bind _lightintensity (Timeline|FireIntensity Play)
    (:Update
      (Rendering|Components|Light|SetIntensity (Variables|Default|GetPointLight) (* _lightintensity (Variables|Default|GetInitialIntensity))))))

(event Collision|EventActorBeginOverlap
  (params (OtherActor :type Actor%20Object%20Reference)))

(event EventTick
  (params (DeltaSeconds :type Float%20%28single-precision%29)))

(fn ConstructionScript
  (Variables|Default|SetInitialIntensity (Variables|/Script/Engine.LightComponentBase|GetIntensity (Variables|Default|GetPointLight))))