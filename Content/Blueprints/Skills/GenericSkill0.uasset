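; GenericSkill0 is a prototype projectile skill, meant to fire ShotsPerSecond shots while held.
; OnPress calls Fire once, which casts to BaseCharacter_BP and has the character spawn GS0_Projectile.
; The looping timer it starts only runs the placeholder smth event, printing "Hello" rather than firing.
; OnRelease clears a differently named timer, tmpfunc, so the smth loop keeps running.
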(event Custom|Fire
  (params (BaseCharacter :type Base%20Character%20Object%20Reference))
  (bind _asbase_character_bp (Utilities|Casting|CastToBaseCharacter_BP BaseCharacter)
    (:then
      (Default|SpawnProjectile _asbase_character_bp "/Game/Blueprints/Skills/GS0_Projectile.GS0_Projectile_C"))
    (:CastFailed
      (Development|PrintString 0 "cast failed"))))

(event Custom|smth
  (Development|PrintString 0))

(event EventOnRelease
  (params (BaseCharacter :type Base%20Character%20Object%20Reference) (PlayerController :type Base%20Player%20Controller%20Object%20Reference))
  ;[1 1 1] Fires ShotsPerSecond shots when pressed and held and stops when released
  (Utilities|Time|ClearTimerbyFunctionName 0 "tmpfunc"))

(event EventOnPress
  (params (BaseCharacter :type Base%20Character%20Object%20Reference) (PlayerController :type Base%20Player%20Controller%20Object%20Reference))
  ;[1 1 1] Fires ShotsPerSecond shots when pressed and held and stops when released
  (CallFunction|Fire BaseCharacter)
  (Utilities|Time|SetTimerbyFunctionName 0 "smth" (/ 1.0 (Variables|Default|GetShotsPerSecond)) true))

(fn ConstructionScript)

(fn Tmpfunc
  (Development|PrintString 0))