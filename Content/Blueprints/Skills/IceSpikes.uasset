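; IceSpikes is a skill actor that raises ice spikes via a Z timeline, then explodes after a set Duration.
; The server times the blast, calls OnExplosion to spawn an avalanche effect and hide the actor without collision, then damages pawns in a box twice the Box extent.
; A short lifespan delays destruction so the explosion multicast reaches all clients.
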(event Custom|OnExplosion
  (Effects|SpawnEmitteratLocation "/Game/StarterContent/Particles/P_Avalanche.P_Avalanche" (+ (Transformation|GetActorLocation) "0, 0,200.000000"))
  (Rendering|SetActorHiddenInGame true)
  (Collision|SetActorEnableCollision false))

(event EventBeginPlay
  (Utilities|FlowControl|Sequence
    (:then_0
      (bind _newtrack_0 (Timeline|SpikesZ Play)
        (:Update
          (Transformation|AddActorLocalOffset (Math|Vector|MakeVector 0.0 0.0 _newtrack_0) false true))))
    (:then_1
      (Networking|SwitchHasAuthority
        (:Authority
          (Utilities|FlowControl|Delay (Variables|Default|GetDuration))
          (CallFunction|OnExplosion)
          (CallFunction|ApplyExplosionDamage)
          ;[1 1 1] We have to give some time so multicast will be called everywheere
          (Actor|SetLifeSpan 2.0))))))

(fn ConstructionScript)

(fn ApplyExplosionDamage
  (bind _box (Variables|Default|GetBox))
  (Networking|SwitchHasAuthority
    (:Authority
      (bind _outactors (Collision|BoxOverlapActors (Transformation|GetWorldLocation _box) (* (Variables|/Script/Engine.BoxComponent|GetBoxExtent _box) 2.0) (Utilities|Array|MakeArray "ObjectTypeQuery3") 0 :!class /Script/Engine.KismetSystemLibrary))
      (for _array_element _outactors
        (Game|Damage|ApplyDamage _array_element (Variables|Default|GetDamageOnExplosion) (Game|GetInstigatorController) 0)))))