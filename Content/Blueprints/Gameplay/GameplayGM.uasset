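; Multiplayer game mode that spawns players as their selected character class and scores frags.
; On login it runs controller setup, waits a fixed delay for player info, copies the name to GameplayPS and respawns the player.
; RespawnPlayer possesses a temporary base character, then SwapCharacter replaces it with the chosen class at a random SpawnVolume point and loads skills.
; Frag prints the kill and adjusts the killer's score, penalizing suicides.
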(event Custom|SwapCharacter
  (params (Character :type Character%20Class%20Reference) (PlayerController :type Player%20Controller%20Object%20Reference))
  (bind _returnvalue (Pawn|GetControlledPawn PlayerController))
  ;[1 1 1] destroys a character already owned by a playercontroller and spawns and possesses a character of a class selected by the player
  (Utilities|IsValid _returnvalue
    (:Is%20Valid
      (Actor|DestroyActor _returnvalue))
    (:Is%20Not%20Valid
      _))
  (bind _returnvalue_2 (Game|SpawnActorfromClass Character (CallFunction|GetRandomSpawnTransform) "Undefined" 0 0))
  (Pawn|Possess PlayerController _returnvalue_2)
  (bind _asbase_character (Utilities|Casting|CastToBaseCharacter _returnvalue_2))
  (Class|BaseCharacter|LoadSkills _asbase_character))

(event Custom|Frag
  (params (Killer :type Controller%20Object%20Reference) (Victim :type Controller%20Object%20Reference))
  (Development|PrintString (Utilities|String|Append (Utilities|String|ToString(Text) (Variables|/Game/Blueprints/Gameplay/BasePlayerControllerBP.BasePlayerControllerBP_C|GetPlayerName (.AsBase%20Player%20Controller%20BP (Utilities|Casting|CastToBasePlayerControllerBP Killer)))) " just killed " (Utilities|String|ToString(Text) (Variables|/Game/Blueprints/Gameplay/BasePlayerControllerBP.BasePlayerControllerBP_C|GetPlayerName (.AsBase%20Player%20Controller%20BP (Utilities|Casting|CastToBasePlayerControllerBP Victim)))) "!!!") true true "(R=0.636097,G=0.000000,B=0.661458,A=1.000000)" 2e+01)
  (if (== Killer Victim)
    (Variables|Default|SetDeltaScore -1)
    (else
      (Variables|Default|SetDeltaScore 1)))
  (Default|ChangeScore (.AsGameplay%20PS (Utilities|Casting|CastToGameplayPS (Variables|/Script/Engine.Controller|GetPlayerState Killer))) (Variables|Default|GetDeltaScore)))

(event Custom|RespawnPlayer
  (params (PlayerController :type Player%20Controller%20Object%20Reference))
  (bind _returnvalue (Pawn|GetControlledPawn PlayerController))
  ;[1 1 1] spawns a base character and makes it owned by the joined playercontroller
  (Utilities|IsValid _returnvalue
    (:Is%20Valid
      (Actor|DestroyActor _returnvalue))
    (:Is%20Not%20Valid
      _))
  (bind _returnvalue_2 (Game|SpawnActorfromClass "/Game/Blueprints/Characters/BaseCharacter_BP.BaseCharacter_BP_C" (CallFunction|GetRandomSpawnTransform) "Undefined" 0 0))
  (Pawn|Possess PlayerController _returnvalue_2)
  (CallFunction|SwapCharacter (.MyPlayerCharacter (Utilities|Struct|BreakPlayerInfo (Variables|/Game/Blueprints/Gameplay/BasePlayerControllerBP.BasePlayerControllerBP_C|GetPlayerInfo (.AsBase%20Player%20Controller%20BP (Utilities|Casting|CastToBasePlayerControllerBP PlayerController))))) PlayerController))

(event EventPostLogin
  (params (NewPlayer :type Player%20Controller%20Object%20Reference))
  (bind _asbase_player_controller_bp (Utilities|Casting|CastToBasePlayerControllerBP NewPlayer))
  ;[1 1 1] initializes spawning a character of a selected class when a player joins
  (Networking|SwitchHasAuthority
    (:Authority
      (Default|InitialSetup _asbase_player_controller_bp)
      ;;[1 1 1] wait for the serverLoadPlayerInfo
      (Utilities|FlowControl|Delay 0.71337)
      (Variables|/Game/Blueprints/Gameplay/GameplayPS.GameplayPS_C|SetName (.AsGameplay%20PS (Utilities|Casting|CastToGameplayPS (Variables|/Script/Engine.Controller|GetPlayerState NewPlayer))) (Variables|/Game/Blueprints/Gameplay/BasePlayerControllerBP.BasePlayerControllerBP_C|GetPlayerName _asbase_player_controller_bp))
      (Default|ClientPostLogin _asbase_player_controller_bp)
      (CallFunction|RespawnPlayer _asbase_player_controller_bp))))

(event EventBeginPlay
  (bind _outactors (Actor|GetAllActorsOfClass "/Game/Blueprints/Environment/SpawnVolume.SpawnVolume_C"))
  (bind _output_get (Variables|Default|SetSpawnVolumes _outactors))
  (Development|PrintString (Utilities|String|ToString(Integer) (Utilities|Array|Length _output_get))))

(fn ConstructionScript)

(fn GetRandomSpawnTransform
  (bind _spawnvolumes (Variables|Default|GetSpawnVolumes))
  (bind _transform (Default|GetRandomSpawnTransform (Utilities|Array|Get(acopy) _spawnvolumes (Math|Random|RandomIntegerinRange 0 (- (Utilities|Array|Length _spawnvolumes) 1)))))
  (Development|PrintString (Utilities|String|ToString(Transform) _transform))
  (return _transform))