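; Game mode for the Boss0 level that spawns each joining player as their selected character.
; On PostLogin, with authority, it runs the player controller's InitialSetup, possesses a temporary base character via RespawnPlayer, then immediately calls SwapCharacter with the class from PlayerInfo.
; Both spawn events destroy the current pawn and spawn at the same hardcoded transform rather than using player starts.
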(event Custom|SwapCharacter
  (params (Character :type Character%20Class%20Reference) (PlayerController :type Player%20Controller%20Object%20Reference))
  (bind _returnvalue (Pawn|GetControlledPawn PlayerController))
  ;[1 1 1] destroys a character already owned by a playercontroller and spawns and possesses a character of a class selected by the player
  (Development|PrintString "SwapCharacter" true true "(R=0.000000,G=0.660000,B=1.000000,A=1.000000)" 1e+01)
  (Utilities|IsValid _returnvalue
    (:Is%20Valid
      (Actor|DestroyActor _returnvalue))
    (:Is%20Not%20Valid
      _))
  (bind _output_get (Variables|Default|SetNewSpawnTransform (Math|Transform|MakeTransform "-1020.000000,-150.000000,112.000000")))
  (bind _returnvalue_2 (Game|SpawnActorfromClass Character _output_get "Undefined" 0 0))
  (Pawn|Possess PlayerController _returnvalue_2))

(event Custom|RespawnPlayer
  (params (PlayerController :type Player%20Controller%20Object%20Reference))
  (bind _returnvalue (Pawn|GetControlledPawn PlayerController))
  ;[1 1 1] spawns a base character and makes it owned by the joined playercontroller
  (Development|PrintString "RespawnPlayer" true true "(R=0.000000,G=0.660000,B=1.000000,A=1.000000)" 1e+01)
  (Utilities|IsValid _returnvalue
    (:Is%20Valid
      (Actor|DestroyActor _returnvalue))
    (:Is%20Not%20Valid
      _))
  (bind _returnvalue_2 (Game|SpawnActorfromClass "/Game/Blueprints/Characters/BaseCharacter_BP.BaseCharacter_BP_C" (Math|Transform|MakeTransform "-1020.000000,-150.000000,112.000000") "Undefined" 0 0))
  (Pawn|Possess PlayerController _returnvalue_2))

(event EventPostLogin
  (params (NewPlayer :type Player%20Controller%20Object%20Reference))
  (bind _asbase_player_controller_bp (Utilities|Casting|CastToBasePlayerControllerBP NewPlayer))
  ;[1 1 1] initializes spawning a character of a selected class when a player joins
  (Networking|SwitchHasAuthority
    (:Authority
      (Development|PrintString "OnPostLogin" true true "(R=0.000000,G=0.660000,B=1.000000,A=1.000000)" 1e+01)
      (Default|InitialSetup _asbase_player_controller_bp)
      (CallFunction|RespawnPlayer _asbase_player_controller_bp)
      (CallFunction|SwapCharacter (.MyPlayerCharacter (Utilities|Struct|BreakPlayerInfo (Variables|/Game/Blueprints/Gameplay/BasePlayerControllerBP.BasePlayerControllerBP_C|GetPlayerInfo _asbase_player_controller_bp))) _asbase_player_controller_bp))))

(fn ConstructionScript)