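; BasePlayerControllerBP is a player controller Blueprint that restores saved player settings during setup.
; An InitialSetup event calls LoadPlayerInfo, which loads the PlayerSettingsSave slot as a PlayerSaveGame and copies its player info struct.
; It then caches the gamepad-use flag and chosen skills on the controller, with debug prints along the way.
; The load stops silently if the save cast fails.
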(event Custom|InitialSetup
  (Development|PrintString "InitialSetup")
  (CallFunction|LoadPlayerInfo))

(fn ConstructionScript)

(fn LoadPlayerInfo
  (bind _returnvalue (SaveGame|LoadGamefromSlot (Variables|Default|GetPlayerSettingsSave)))
  (bind _asplayer_save_game (Utilities|Casting|CastToPlayerSaveGame _returnvalue))
  (bind _output_get (Variables|Default|SetPlayerInfo (Variables|/Game/Blueprints/AllLevels/PlayerSaveGame.PlayerSaveGame_C|GetS_PlayerInfo _asplayer_save_game)))
  (Variables|Default|SetbIsUsingPad (.UsingPad (Utilities|Struct|BreakPlayerInfo _output_get)))
  (Variables|Default|SetSkills (.ChosenSkills (Utilities|Struct|BreakPlayerInfo _output_get)))
  (Development|PrintString "bpc skills are set"))